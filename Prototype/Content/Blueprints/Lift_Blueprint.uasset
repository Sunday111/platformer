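; Lift Blueprint for a sprite platform that shuttles between its origin and EndLocation once LiftForward is called.
; LiftTimeline drives the position lerp, and on finish waits StopDelaySeconds before running the opposite way.
; A Box overlap flips the travel direction, guarded by Overlapped against repeats until the overlap ends.
; The construction script applies the sprite color, derives play rate from TravelTimeSeconds, and can preview the end position via TestEndLocation.
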(event OnComponentBeginOverlap(Box)
  (params (OverlappedComponent :type Primitive%20Component%20Object%20Reference) (OtherActor :type Actor%20Object%20Reference) (OtherComp :type Primitive%20Component%20Object%20Reference) (OtherBodyIndex :type Integer) (bFromSweep :type Boolean) (SweepResult :type Hit%20Result%20Structure%20%28by%20ref%29))
  (bind _lift_timeline (Variables|Default|GetLift%20Timeline))
  ;[1 1 1] Handle Collisions
  (Utilities|FlowControl|Sequence
    (:then_0
      (if (not (Variables|Default|GetOverlapped))
        (if (Class|TimelineComponent|IsReversing _lift_timeline)
          (Audio|Components|Audio|Play _lift_timeline)
          (else
            (Utilities|String|Reverse _lift_timeline)))))
    (:then_1
      (Variables|Default|SetOverlapped true))))

(event OnComponentEndOverlap(Box)
  (params (OverlappedComponent :type Primitive%20Component%20Object%20Reference) (OtherActor :type Actor%20Object%20Reference) (OtherComp :type Primitive%20Component%20Object%20Reference) (OtherBodyIndex :type Integer))
  ;[1 1 1] Handle Collisions
  (Variables|Default|SetOverlapped false))

(event Custom|Lift%20Back
  (bind (_direction _lerp_alpha) (Timeline|Lift%20Timeline ReverseFromEnd)
    (:Update
      (Transformation|SetRelativeLocation (Variables|Default|GetLift%20Sprite) (Math|Vector|Lerp(Vector) "0, 0, 0" (Variables|LiftControls|GetEnd%20Location) _lerp_alpha) false false))
    (:Finished
      (Utilities|FlowControl|Delay (Variables|LiftControls|GetStop%20Delay%20%28seconds%29))
      (switch Utilities|FlowControl|Switch|SwitchonETimelineDirection _direction
        (:Forward
          (CallFunction|LiftBack))
        (:Backward
          (CallFunction|LiftForward))))))

(event Custom|Lift%20Forward
  (bind (_direction _lerp_alpha) (Timeline|Lift%20Timeline PlayFromStart)
    (:Update
      (Transformation|SetRelativeLocation (Variables|Default|GetLift%20Sprite) (Math|Vector|Lerp(Vector) "0, 0, 0" (Variables|LiftControls|GetEnd%20Location) _lerp_alpha) false false))
    (:Finished
      (Utilities|FlowControl|Delay (Variables|LiftControls|GetStop%20Delay%20%28seconds%29))
      (switch Utilities|FlowControl|Switch|SwitchonETimelineDirection _direction
        (:Forward
          (CallFunction|LiftBack))
        (:Backward
          (CallFunction|LiftForward))))))

(event EventBeginPlay)

(event Collision|EventActorBeginOverlap
  (params (OtherActor :type Actor%20Object%20Reference)))

(event EventTick
  (params (DeltaSeconds :type Float%20%28single-precision%29)))

(fn ConstructionScript
  (Utilities|FlowControl|Sequence
    (:then_0
      (Transformation|SetRelativeLocation (Variables|Default|GetLift%20Sprite) (Math|Vector|SelectVector (Variables|LiftControls|GetEnd%20Location) "0, 0, 0" (Variables|LiftControls|GetTest%20end%20location)) false true))
    (:then_1
      (Sprite|SetSpriteColor (Variables|Default|GetLift%20Sprite) (Variables|LiftControls|GetColor)))
    (:then_2
      (Components|Timeline|SetPlayRate (Variables|Default|GetLift%20Timeline) (/ 1.0 (Variables|LiftControls|GetTravel%20Time%20%28Seconds%29))))))