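; Paper2D character Blueprint that picks the sprite animation to match the character's movement.
; The AnimationUpdate event derives moving and falling flags from velocity and the CharacterMovement component, then sets the Sprite's flipbook from the result.
; A simple state machine function gives falling priority over running, defaults to idle, and maps the chosen state to its flipbook with a Select.
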(event EventAnimationUpdate
  (bind _flipbook (CallFunction|AnimationStateMachine (> (Math|Vector|VectorLengthSquared (Transformation|GetVelocity)) 0.0) (AI|Components|NavMovement|IsFalling (Variables|Character|GetCharacterMovement))))
  (Sprite|SetFlipbook (Variables|Default|GetSprite) _flipbook))

(fn ConstructionScript)

(fn AnimationStateMachine
  (params (IsMoving :type Boolean) (IsFalling :type Boolean))
  ;[1 1 1] Input
  (LocalVariables|SetIs_Moving_Local IsMoving)
  (LocalVariables|SetIs_Falling_Local IsFalling)
  (if (LocalVariables|GetIs_Falling_Local)
    (LocalVariables|SetAnimation_State "NewEnumerator2")
    (elif (LocalVariables|GetIs_Moving_Local)
      (LocalVariables|SetAnimation_State "NewEnumerator1")
      (else
        (LocalVariables|SetAnimation_State "NewEnumerator0"))))
  (return (Utilities|Select :Index (LocalVariables|GetAnimation_State) :NewEnumerator0 (Variables|Animations|GetIdle) :NewEnumerator1 (Variables|Animations|GetRun) :NewEnumerator2 (Variables|Animations|GetFalling))))